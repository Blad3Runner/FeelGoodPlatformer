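; BP_Crystal is an elemental crystal collectable that adds one Water, Fire, Air or Thunder stone to the player's data.
; CanBePickedUp always allows pickup, and the event graph holds no active logic.
; ApplyToPlayerData rebuilds the player struct, using Selects on BoostType to increment the matching stone count and copying the other fields through.
; The Earth type increments nothing and resets Air and Thunder stones to zero.
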(fn `ApplyToPlayerData`
  (params (SPlayerDataIn :type "/Game/Blueprints/Libraries/Structs/SPlayerData Structure"))
  (returns (SPlayerDataOut :type "/Game/Blueprints/Libraries/Structs/SPlayerData Structure"))
  (bind ((`WaterStones_75_E87C5C0D41D11715B1BED9AD952F7DDA` _waterstones)) (break `/Game/Blueprints/Libraries/Structs/SPlayerData` SPlayerDataIn))
  (bind ((`WaterStones_75_E87C5C0D41D11715B1BED9AD952F7DDA` _waterstones_2) (`FireStones_76_946E0739440000FF9DC13F9B0BCD0674` _firestones)) (break `/Game/Blueprints/Libraries/Structs/SPlayerData` SPlayerDataIn))
  (bind ((`WaterStones_75_E87C5C0D41D11715B1BED9AD952F7DDA` _waterstones_3) (`FireStones_76_946E0739440000FF9DC13F9B0BCD0674` _firestones_2) (`AirStones_77_C4AE268E40DF86A382ADA5A6B5353E6D` _airstones)) (break `/Game/Blueprints/Libraries/Structs/SPlayerData` SPlayerDataIn))
  (bind ((`BaseSpeed_18_F3C2D458437A1703049EE1BE10DF69DF` _basespeed) (`CurrentHealth_22_A69C23BC42BEAC963CE56F9FC396565D` _currenthealth) (`MaxHealth_24_392580E8455509ED2F7D1789E3B74822` _maxhealth) (`ElectricResistance_25_EA641BED40F78FC10F8099BBCA6FBC1D` _electricresistance) (`FireResistance_26_960FC6914719D036A96713BC45313C4D` _fireresistance) (`WaterResistance_27_407BFA37470805D076160D8815FCA1C3` _waterresistance) (`AirResistance_28_9E5B853340D37B019D0D3DB71544A8C8` _airresistance) (`BaseDamage_29_0179021543C94CB6E4DDECB08D1F143E` _basedamage) (`JumpHeight_30_1ADE76854E76A5E1AEFFD3A7F5AA82AD` _jumpheight) (`JumpDistance_31_76F57A5F45B6BC06AA3335B8270076AE` _jumpdistance) (`FireDamage_40_09DFD62A426215518C78269FF86D4995` _firedamage) (`WaterDamage_41_D379DE884C8590C9178508AC96FBBDDE` _waterdamage) (`ElectricDamage_44_EC110E4A47B381732A559282D8A478E9` _electricdamage) (`AirDamage_45_1C3683414E6DC6728A36B48449B73E91` _airdamage) (`MaxElementalResistance_48_4DBE1B0C41D2713E7A8BF4BC123D8415` _maxelementalresistance) (`ParryTime_51_767A0A5B45A558FB3B4581A8CC98B27E` _parrytime) (`MaxSpeed_53_1D2FB8754C19E8B474D2DBB9BCB55634` _maxspeed) (`MaxJumpDistance_55_582ABA0A4322CE17564F888482B7CD2B` _maxjumpdistance) (`MaxParryTime_57_5A41DFDF491321C223D9F1A662E4162A` _maxparrytime) (`MaxDamage_59_CD07F212414728E28E34D5B91950C8A1` _maxdamage) (`MaxJumps_62_13472EF34751F2FDE3F329A559A3F670` _maxjumps) (`JumpsNumber_64_536B74004F52A316E64EA1968FA73C79` _jumpsnumber) (`Mortars_79_258811CD4E0B1FFE03C0F5A1D7673277` _mortars)) (break `/Game/Blueprints/Libraries/Structs/SPlayerData` SPlayerDataIn))
  (bind ((`WaterStones_75_E87C5C0D41D11715B1BED9AD952F7DDA` _waterstones_4) (`FireStones_76_946E0739440000FF9DC13F9B0BCD0674` _firestones_3) (`AirStones_77_C4AE268E40DF86A382ADA5A6B5353E6D` _airstones_2) (`ThunderStones_78_E414D64C4BF32BA61F83069ED042F73C` _thunderstones)) (break `/Game/Blueprints/Libraries/Structs/SPlayerData` SPlayerDataIn))
  (return (make `/Game/Blueprints/Libraries/Structs/SPlayerData` _basespeed _currenthealth _maxhealth _electricresistance _fireresistance _waterresistance _airresistance _basedamage _jumpheight _jumpdistance _firedamage _waterdamage _electricdamage _airdamage _maxelementalresistance _parrytime _maxspeed _maxjumpdistance _maxparrytime _maxdamage _maxjumps _jumpsnumber (select `/Game/Blueprints/Libraries/Enums/E_ElementType` (`self.BoostType`) :`NewEnumerator0` _waterstones :`NewEnumerator1` _waterstones :`NewEnumerator2` (+ _waterstones 1) :`NewEnumerator3` _waterstones :`NewEnumerator4` _waterstones) (select `/Game/Blueprints/Libraries/Enums/E_ElementType` (`self.BoostType`) :`NewEnumerator0` (+ _firestones 1) :`NewEnumerator1` _firestones :`NewEnumerator2` _firestones :`NewEnumerator3` _firestones :`NewEnumerator4` _firestones) (select `/Game/Blueprints/Libraries/Enums/E_ElementType` (`self.BoostType`) :`NewEnumerator0` _airstones :`NewEnumerator1` (+ _airstones 1) :`NewEnumerator2` _airstones :`NewEnumerator3` _airstones) (select `/Game/Blueprints/Libraries/Enums/E_ElementType` (`self.BoostType`) :`NewEnumerator0` _thunderstones :`NewEnumerator1` _thunderstones :`NewEnumerator2` _thunderstones :`NewEnumerator3` (+ _thunderstones 1)) _mortars)))

(fn `CanBePickedUp`
  (params (Character :type "/Game/ThirdPerson/Blueprints/BP_ThirdPersonCharacter Object Reference"))
  (returns (CanBePickedUp :type Boolean))
  (return true))

(fn `UserConstructionScript`
  (`parent.UserConstructionScript`))