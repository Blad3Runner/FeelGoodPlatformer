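; Base actor for collectable pickups, with a floating mesh that plays an optional sound and destroys itself on Interact.
; The construction script tints the mesh through a dynamic material instance using the Color variable.
; On BeginPlay, a timeline scaled by FloatingSpeed lerps the mesh's relative height to animate it.
; CanBePickedUp always returns true and ApplyToPlayerData is an empty stub, neither called here.
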(event `self.ReceiveBeginPlay`
  (bind (_collectablerelativelocation_x _collectablerelativelocation_y _collectablerelativelocation_z) (`KismetMathLibrary.BreakVector` (`self.CollectableRelativeLocation`)))
  (`TimelineComponent.SetPlayRate` (`self.Timeline`) (`self.FloatingSpeed`))
  (set `self.CollectableRelativeLocation` (`SceneComponent.RelativeLocation` (`self.StaticMesh`)))
  (bind (_direction _animationalpha) (`Timeline|Timeline`)
    (:`Update`
      (`SceneComponent.K2_SetRelativeLocation` (`self.StaticMesh`) (`KismetMathLibrary.VLerp` (`self.CollectableRelativeLocation`) (`KismetMathLibrary.MakeVector` _collectablerelativelocation_x _collectablerelativelocation_y (+ _collectablerelativelocation_z 50.0)) _animationalpha) false false))))

(event `/Game/Blueprints/Interfaces/BPI_Interaction.Interact`
  (params (Instigator :type "Actor Object Reference"))
  (bind _pickupsound (`self.PickupSound`)
    (:`then`
      (`GameplayStatics.PlaySoundAtLocation` _pickupsound (`SceneComponent.K2_GetComponentLocation` (`self.StaticMesh`)) (struct) 1.0 1.0 0.0 null null null null))
    (:`else`
      _))
  (`self.K2_DestroyActor`))

(fn `ApplyToPlayerData`
  (params (SPlayerDataIn :type "/Game/Blueprints/Libraries/Structs/SPlayerInfo Structure"))
  (returns (SPlayerDataOut :type "/Game/Blueprints/Libraries/Structs/SPlayerInfo Structure"))
  (return))

(fn `CanBePickedUp`
  (params (Character :type "/Game/ThirdPerson/Blueprints/BP_ThirdPersonCharacter Object Reference"))
  (returns (CanBePickedUp :type Boolean))
  (return true))

(fn `UserConstructionScript`
  (bind _returnvalue (`PrimitiveComponent.CreateDynamicMaterialInstance` (`self.StaticMesh`) 0 "/Game/Blueprints/Collectables/Assets/Materials/M_Collectable_Inst.M_Collectable_Inst" "None"))
  (bind _output_get (set `self.Material` _returnvalue))
  (`MaterialInstanceDynamic.SetVectorParameterValue` _output_get "Color" (`self.Color`)))