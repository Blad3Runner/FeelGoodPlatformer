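; Base collectable shield that raises one of the player's elemental resistances, chosen by ShieldType.
; CanBePickedUp reads player 0's character, ignoring its Character input, and allows pickup while that resistance is below MaxElementalResistance.
; ApplyToPlayerData returns rebuilt player data with ResistanceBonus added to the matching resistance, without clamping.
; Earth has no pickup case, and its selects zero all four resistances.
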(fn `ApplyToPlayerData`
  (params (SPlayerDataIn :type "/Game/Blueprints/Libraries/Structs/SPlayerData Structure"))
  (returns (SPlayerDataOut :type "/Game/Blueprints/Libraries/Structs/SPlayerData Structure"))
  (bind (_basespeed _currenthealth _maxhealth _electricresistance _fireresistance _waterresistance _airresistance _basedamage _jumpheight _jumpdistance _firedamage _waterdamage _electricdamage _airdamage _maxelementalresistance _parrytime _maxspeed _maxjumpdistance _maxparrytime _maxdamage _maxjumps _jumpsnumber _waterstones _firestones _airstones _thunderstones _mortars) (break `/Game/Blueprints/Libraries/Structs/SPlayerData` SPlayerDataIn))
  (bind _resistancebonus (`self.ResistanceBonus`))
  (bind _shieldtype (`self.ShieldType`))
  (return (make `/Game/Blueprints/Libraries/Structs/SPlayerData` _basespeed _currenthealth _maxhealth (select `/Game/Blueprints/Libraries/Enums/E_ElementType` _shieldtype :`NewEnumerator0` _electricresistance :`NewEnumerator1` _electricresistance :`NewEnumerator2` _electricresistance :`NewEnumerator3` (+ _electricresistance _resistancebonus)) (select `/Game/Blueprints/Libraries/Enums/E_ElementType` _shieldtype :`NewEnumerator0` (+ _fireresistance _resistancebonus) :`NewEnumerator1` _fireresistance :`NewEnumerator2` _fireresistance :`NewEnumerator3` _fireresistance) (select `/Game/Blueprints/Libraries/Enums/E_ElementType` _shieldtype :`NewEnumerator0` _waterresistance :`NewEnumerator1` _waterresistance :`NewEnumerator2` (+ _waterresistance _resistancebonus) :`NewEnumerator3` _waterresistance) (select `/Game/Blueprints/Libraries/Enums/E_ElementType` _shieldtype :`NewEnumerator0` _airresistance :`NewEnumerator1` (+ _airresistance _resistancebonus) :`NewEnumerator2` _airresistance :`NewEnumerator3` _airresistance) _basedamage _jumpheight _jumpdistance _firedamage _waterdamage _electricdamage _airdamage _maxelementalresistance _parrytime _maxspeed _maxjumpdistance _maxparrytime _maxdamage _maxjumps _jumpsnumber _waterstones _firestones _airstones _thunderstones _mortars)))

(fn `CanBePickedUp`
  (params (Character :type "/Game/ThirdPerson/Blueprints/BP_ThirdPersonCharacter Object Reference"))
  (returns (CanBePickedUp :type Boolean))
  (bind _asbp_third_person_character (cast `/Game/ThirdPerson/Blueprints/BP_ThirdPersonCharacter` (`GameplayStatics.GetPlayerCharacter` 0)))
  (switch `/Game/Blueprints/Libraries/Enums/E_ElementType` (`self.ShieldType`)
    (:`NewEnumerator0`
      (bind _splayerdata (`/Game/ThirdPerson/Blueprints/BP_ThirdPersonCharacter.SPlayerData` _asbp_third_person_character))
      (bind ((`ElectricResistance_25_EA641BED40F78FC10F8099BBCA6FBC1D` _electricresistance) (`FireResistance_26_960FC6914719D036A96713BC45313C4D` _fireresistance) (`WaterResistance_27_407BFA37470805D076160D8815FCA1C3` _waterresistance) (`AirResistance_28_9E5B853340D37B019D0D3DB71544A8C8` _airresistance)) (break `/Game/Blueprints/Libraries/Structs/SPlayerData` _splayerdata))
      (bind ((`MaxElementalResistance_48_4DBE1B0C41D2713E7A8BF4BC123D8415` _maxelementalresistance)) (break `/Game/Blueprints/Libraries/Structs/SPlayerData` _splayerdata))
      (if (< _fireresistance _maxelementalresistance)
        (return true)
        (else
          (return false))))
    (:`NewEnumerator1`
      (if (< _airresistance _maxelementalresistance)
        (return true)
        (else
          (return false))))
    (:`NewEnumerator2`
      (if (< _waterresistance _maxelementalresistance)
        (return true)
        (else
          (return false))))
    (:`NewEnumerator3`
      (if (< _electricresistance _maxelementalresistance)
        (return true)
        (else
          (return false))))))

(fn `UserConstructionScript`
  (`parent.UserConstructionScript`))