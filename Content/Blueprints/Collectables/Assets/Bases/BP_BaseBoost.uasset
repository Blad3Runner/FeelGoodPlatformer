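; Base collectable boost that raises one player stat chosen by BoostType: jump distance, jump count, damage, parry time or speed.
; CanBePickedUp allows pickup only while that stat is below its maximum, reading player 0's character instead of the Character input.
; ApplyToPlayerData returns a rebuilt SPlayerInfo, using Selects to multiply the chosen stat by its bonus, or add it for jump count, without clamping.
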(fn `ApplyToPlayerData`
  (params (SPlayerDataIn :type "/Game/Blueprints/Libraries/Structs/SPlayerInfo Structure"))
  (returns (SPlayerDataOut :type "/Game/Blueprints/Libraries/Structs/SPlayerInfo Structure"))
  (bind ((`JumpsNumber_76_903D1D80495F2CED340E2C88D09809A4` _jumpsnumber)) (break `/Game/Blueprints/Libraries/Structs/SPlayerInfo` SPlayerDataIn))
  (bind ((`ParryTime_70_755AB6DB48CB11441AE7EC9D44D641E0` _parrytime)) (break `/Game/Blueprints/Libraries/Structs/SPlayerInfo` SPlayerDataIn))
  (bind (_basespeed _currenthealth _maxhealth _electricresistance _fireresistance _waterresistance _airresistance _basedamage _jumpheight _jumpdistance _firedamage _waterdamage _electricdamage _airdamage _maxelementalresistance _parrytime_2 _maxspeed _maxjumpdistance _maxparrytime _maxdamage _jumpsnumber_2 _maxjumps _waterstones _firestones _airstones _thunderstones _mortars) (break `/Game/Blueprints/Libraries/Structs/SPlayerInfo` SPlayerDataIn))
  (bind ((`BaseSpeed_55_DFA912A2405E6CAB10D378AC5F8A3371` _basespeed_2)) (break `/Game/Blueprints/Libraries/Structs/SPlayerInfo` SPlayerDataIn))
  (bind ((`BaseDamage_62_3DE90C2D4D814519BE2FD1B997C8C0BE` _basedamage_2)) (break `/Game/Blueprints/Libraries/Structs/SPlayerInfo` SPlayerDataIn))
  (bind ((`JumpDistance_64_B52F7AF544C0B27D330A9E850F821F8E` _jumpdistance_2)) (break `/Game/Blueprints/Libraries/Structs/SPlayerInfo` SPlayerDataIn))
  (return (make `/Game/Blueprints/Libraries/Structs/SPlayerInfo` (select `/Game/Blueprints/Libraries/Enums/E_BoostType` (`self.BoostType`) :`NewEnumerator0` _basespeed_2 :`NewEnumerator1` _basespeed_2 :`NewEnumerator2` _basespeed_2 :`NewEnumerator3` _basespeed_2 :`NewEnumerator4` (* _basespeed_2 (`self.SpeedBonus`))) _currenthealth _maxhealth _electricresistance _fireresistance _waterresistance _airresistance (select `/Game/Blueprints/Libraries/Enums/E_BoostType` (`self.BoostType`) :`NewEnumerator0` _basedamage_2 :`NewEnumerator1` _basedamage_2 :`NewEnumerator2` (* _basedamage_2 (`self.DamageBonus`)) :`NewEnumerator3` _basedamage_2 :`NewEnumerator4` _basedamage_2) _jumpheight (select `/Game/Blueprints/Libraries/Enums/E_BoostType` (`self.BoostType`) :`NewEnumerator0` (* _jumpdistance_2 (`self.JumpDistanceBonus`)) :`NewEnumerator1` _jumpdistance_2 :`NewEnumerator2` _jumpdistance_2 :`NewEnumerator3` _jumpdistance_2 :`NewEnumerator4` _jumpdistance_2) _firedamage _waterdamage _electricdamage _airdamage _maxelementalresistance (select `/Game/Blueprints/Libraries/Enums/E_BoostType` (`self.BoostType`) :`NewEnumerator0` _parrytime :`NewEnumerator1` _parrytime :`NewEnumerator2` _parrytime :`NewEnumerator3` (* _parrytime (`self.ParryTimeBonus`)) :`NewEnumerator4` _parrytime) _maxspeed _maxjumpdistance _maxparrytime _maxdamage (`KismetMathLibrary.FTrunc` (select `/Game/Blueprints/Libraries/Enums/E_BoostType` (`self.BoostType`) :`NewEnumerator0` (`KismetMathLibrary.Conv_IntToDouble` _jumpsnumber) :`NewEnumerator1` (`KismetMathLibrary.Conv_IntToDouble` (+ _jumpsnumber (`self.JumpsNumberBonus`))) :`NewEnumerator2` (`KismetMathLibrary.Conv_IntToDouble` _jumpsnumber) :`NewEnumerator3` (`KismetMathLibrary.Conv_IntToDouble` _jumpsnumber) :`NewEnumerator4` (`KismetMathLibrary.Conv_IntToDouble` _jumpsnumber))) _maxjumps _waterstones _firestones _airstones _thunderstones _mortars)))

(fn `CanBePickedUp`
  (params (Character :type "/Game/ThirdPerson/Blueprints/BP_ThirdPersonCharacter Object Reference"))
  (returns (CanBePickedUp :type Boolean))
  (bind _asbp_third_person_character (cast `/Game/ThirdPerson/Blueprints/BP_ThirdPersonCharacter` (`GameplayStatics.GetPlayerCharacter` 0)))
  (switch `/Game/Blueprints/Libraries/Enums/E_BoostType` (`self.BoostType`)
    (:`NewEnumerator0`
      (bind _splayerinfo (`/Game/ThirdPerson/Blueprints/BP_ThirdPersonCharacter.SPlayerInfo` _asbp_third_person_character))
      (bind ((`BaseSpeed_55_DFA912A2405E6CAB10D378AC5F8A3371` _basespeed) (`BaseDamage_62_3DE90C2D4D814519BE2FD1B997C8C0BE` _basedamage) (`JumpDistance_64_B52F7AF544C0B27D330A9E850F821F8E` _jumpdistance) (`ParryTime_70_755AB6DB48CB11441AE7EC9D44D641E0` _parrytime) (`JumpsNumber_76_903D1D80495F2CED340E2C88D09809A4` _jumpsnumber)) (break `/Game/Blueprints/Libraries/Structs/SPlayerInfo` _splayerinfo))
      (bind ((`MaxSpeed_71_0D7AFD334804D6B278D063A14DF4A84B` _maxspeed) (`MaxJumpDistance_73_D9862289435DABB5175A9887921F8106` _maxjumpdistance) (`MaxParryTime_74_233003364D9BAD37C106619308285615` _maxparrytime) (`MaxDamage_75_D2E46CC34BF830B7B9957FBB9101653E` _maxdamage) (`MaxJumps_77_36CAE47241774D2A6F80E49CF023D834` _maxjumps)) (break `/Game/Blueprints/Libraries/Structs/SPlayerInfo` _splayerinfo))
      (if (< _jumpdistance _maxjumpdistance)
        (return true)
        (else
          (return false))))
    (:`NewEnumerator1`
      (if (< _jumpsnumber _maxjumps)
        (return true)
        (else
          (return false))))
    (:`NewEnumerator2`
      (if (< _basedamage _maxdamage)
        (return true)
        (else
          (return false))))
    (:`NewEnumerator3`
      (if (< _parrytime _maxparrytime)
        (return true)
        (else
          (return false))))
    (:`NewEnumerator4`
      (if (< _basespeed _maxspeed)
        (return true)
        (else
          (return false))))))

(fn `UserConstructionScript`
  (`parent.UserConstructionScript`))