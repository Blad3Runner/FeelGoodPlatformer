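; Base Blueprint for an elemental collectable, which by its name relates to elemental damage and can always be picked up.
; ApplyToPlayerData has an empty body, with an unreached return node that would rebuild the player data struct.
; That disconnected logic uses BoostType to increment Water, Fire, Air or Thunder stones and copies the other stats.
; Its Earth case zeroes Air and Thunder stones.
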(fn `ApplyToPlayerData`
  (params (SPlayerDataIn :type "/Game/Blueprints/Libraries/Structs/SPlayerInfo Structure"))
  (returns (SPlayerDataOut :type "/Game/Blueprints/Libraries/Structs/SPlayerInfo Structure")))

(fn `CanBePickedUp`
  (params (Character :type "/Game/ThirdPerson/Blueprints/BP_ThirdPersonCharacter Object Reference"))
  (returns (CanBePickedUp :type Boolean))
  (return true))

(fn `UserConstructionScript`
  (`parent.UserConstructionScript`))