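; Base health collectable that either restores the player's HP or raises max HP, depending on HeartType.
; CanBePickedUp overrides the parent to allow pickup only when player 0 is below max health, for both types, ignoring its Character input.
; ApplyToPlayerData rebuilds the player data struct, changing only health fields.
; Restoring clamps to MaxHealth plus HealthExtension, while increasing max leaves current health unchanged.
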(fn `ApplyToPlayerData`
  (params (SPlayerDataIn :type "/Game/Blueprints/Libraries/Structs/SPlayerData Structure"))
  (returns (SPlayerDataOut :type "/Game/Blueprints/Libraries/Structs/SPlayerData Structure"))
  (bind (_basespeed _currenthealth _maxhealth _electricresistance _fireresistance _waterresistance _airresistance _basedamage _jumpheight _jumpdistance _firedamage _waterdamage _electricdamage _airdamage _maxelementalresistance _parrytime _maxspeed _maxjumpdistance _maxparrytime _maxdamage _maxjumps _jumpsnumber _waterstones _firestones _airstones _thunderstones _mortars) (break `/Game/Blueprints/Libraries/Structs/SPlayerData` SPlayerDataIn))
  (bind _hearttype (`self.HeartType`))
  (bind _returnvalue (+ _maxhealth (`self.HealthExtension`)))
  (return (make `/Game/Blueprints/Libraries/Structs/SPlayerData` _basespeed (select `/Game/Blueprints/Libraries/Enums/E_HeartType` _hearttype :`NewEnumerator0` (`KismetMathLibrary.Clamp` (+ (`self.HealthRecovery`) _currenthealth) 0 _returnvalue) :`NewEnumerator1` _currenthealth) (select `/Game/Blueprints/Libraries/Enums/E_HeartType` _hearttype :`NewEnumerator0` _maxhealth :`NewEnumerator1` _returnvalue) _electricresistance _fireresistance _waterresistance _airresistance _basedamage _jumpheight _jumpdistance _firedamage _waterdamage _electricdamage _airdamage _maxelementalresistance _parrytime _maxspeed _maxjumpdistance _maxparrytime _maxdamage _maxjumps _jumpsnumber _waterstones _firestones _airstones _thunderstones _mortars)))

(fn `CanBePickedUp`
  (params (Character :type "/Game/ThirdPerson/Blueprints/BP_ThirdPersonCharacter Object Reference"))
  (returns (CanBePickedUp :type Boolean))
  (bind _asbp_third_person_character (cast `/Game/ThirdPerson/Blueprints/BP_ThirdPersonCharacter` (`GameplayStatics.GetPlayerCharacter` 0))
    (:`then`
      (bind ((`CurrentHealth_22_A69C23BC42BEAC963CE56F9FC396565D` _currenthealth) (`MaxHealth_24_392580E8455509ED2F7D1789E3B74822` _maxhealth)) (break `/Game/Blueprints/Libraries/Structs/SPlayerData` (`/Game/ThirdPerson/Blueprints/BP_ThirdPersonCharacter.SPlayerData` _asbp_third_person_character)))
      (if (< _currenthealth _maxhealth)
        (return true)
        (else
          (return false))))
    (:`CastFailed`
      (return false))))

(fn `UserConstructionScript`
  (`parent.UserConstructionScript`))